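; Player Blueprint that handles first-person looking and movement, with support for VR headsets.
; Look axes are scaled by sensitivity and frame time, while movement follows the camera's direction when an HMD is enabled, otherwise the actor's.
; An input toggles a right-hand extended flag; no input here sets the left.
; Tick sphere-traces forward from the camera whatever the hand flags, but the hit result is not yet used.
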(event `InputAxis|HeadTurnLeft`
  (params (AxisValue :type "Float (single-precision)"))
  ;[1 1 1] HandleLooking
  (`self.AddControllerYawInput` (`KismetMathLibrary.BreakVector2D` (* (* (`KismetMathLibrary.MakeVector2D` AxisValue (stale `InputAxis|HeadTurnUp` AxisValue)) (`self.Sensitivity`)) (`GameplayStatics.GetWorldDeltaSeconds`)))))

(event `InputAxis|HeadTurnUp`
  (params (AxisValue :type "Float (single-precision)"))
  ;[1 1 1] HandleLooking
  (`self.AddControllerPitchInput` (`.Y` (`KismetMathLibrary.BreakVector2D` (* (* (`KismetMathLibrary.MakeVector2D` (stale `InputAxis|HeadTurnLeft` AxisValue) AxisValue) (`self.Sensitivity`)) (`GameplayStatics.GetWorldDeltaSeconds`))))))

(event `InputAxis|MovementBackForward`
  (params (AxisValue :type "Float (single-precision)"))
  ;[1 1 1] Movement
  ;;[1 1 1] Handle Forward/Backward Movement
  (`self.AddMovementInput` (select `bool` (`HeadMountedDisplayFunctionLibrary.IsHeadMountedDisplayEnabled`) :`false` (`self.GetActorForwardVector`) :`true` (`SceneComponent.GetForwardVector` (`self.Camera`))) (+ AxisValue (stale `InputAxisKey|Gamepad_LeftY` AxisValue)) :!label _label))

(event `InputAxisKey|Gamepad_LeftY`
  (params (AxisValue :type "Float (single-precision)"))
  ;[1 1 1] Movement
  ;;[1 1 1] Handle Forward/Backward Movement
  (goto _label))

(event `InputAxisKey|Gamepad_LeftX`
  (params (AxisValue :type "Float (single-precision)"))
  ;[1 1 1] Movement
  ;;[1 1 1] Handle Right/Left Movement
  (`self.AddMovementInput` (select `bool` (`HeadMountedDisplayFunctionLibrary.IsHeadMountedDisplayEnabled`) :`false` (`self.GetActorRightVector`) :`true` (`SceneComponent.GetRightVector` (`self.Camera`))) (+ AxisValue (stale `InputAxis|MovementLeft/Right` AxisValue)) :!label _label_2))

(event `InputAxis|MovementLeft/Right`
  (params (AxisValue :type "Float (single-precision)"))
  ;[1 1 1] Movement
  ;;[1 1 1] Handle Right/Left Movement
  (goto _label_2))

(event `InputAction|ExtendLeft`
  (params (Key :type "Key Structure"))
  ;[1 1 1] handling booleans for extending hands
)

(event `InputAction|ExtendRight`
  (params (Key :type "Key Structure"))
  ;[1 1 1] handling booleans for extending hands
  (:`Pressed`
    (set `self.RightExtended` (not (`self.RightExtended`)))))

(event `self.ReceiveTick`
  (params (DeltaSeconds :type "Float (single-precision)"))
  (if (and (`self.LeftExtended`) (`self.RightExtended`))
    (`self.CastFromCam` 0.0)
    (if (`self.LeftExtended`)
      _)
    (else
      (`self.CastFromCam` 0.0)
      (if (`self.RightExtended`)
        _))))

(fn `CastFromCam`
  (params (Radius :type "Float (double-precision)") (Distance :type "Float (double-precision)") (ComplexTrace :type Boolean) (DrawDebug :type Boolean))
  (returns (Hit :type "HitResult Structure"))
  (bind _camera (`self.Camera`))
  (bind _returnvalue (`SceneComponent.K2_GetComponentLocation` _camera))
  (bind _outhit (`KismetSystemLibrary.SphereTraceSingle` :`Start` _returnvalue :`End` (+ _returnvalue (* (`KismetMathLibrary.GetForwardVector` (`SceneComponent.K2_GetComponentRotation` _camera)) Distance)) :`Radius` Radius :`TraceChannel` "TraceTypeQuery1" :`bTraceComplex` ComplexTrace :`DrawDebugType` (select `bool` DrawDebug :`true` "ForOneFrame" :!type "EDrawDebugTrace Enum")))
  (return _outhit))

(fn `UserConstructionScript`)