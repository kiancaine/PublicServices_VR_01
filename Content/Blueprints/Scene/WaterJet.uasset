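; Water jet scene actor that puts out FireOld actors in its path while active.
; Every tick it syncs the Water component's activation to the Active flag.
; When active, it sphere-traces on the Visibility channel along its forward vector out to Range and sets a hit FireOld's Active to false.
; The trace still has debug drawing enabled.
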(event `self.ReceiveTick`
  (params (DeltaSeconds :type "Float (single-precision)"))
  (bind _returnvalue (`self.K2_GetActorLocation`))
  (bind _active (`self.Active`))
  (`|ExecutionSequence`
    (:`then_0`
      (`ActorComponent.SetActive` (`self.Water`) _active false))
    (:`then_1`
      (if _active
        (bind _outhit (`KismetSystemLibrary.SphereTraceSingle` :`Start` _returnvalue :`End` (+ _returnvalue (* (`KismetMathLibrary.GetForwardVector` (`self.K2_GetActorRotation`)) (`self.Range`))) :`TraceChannel` "TraceTypeQuery1" :`DrawDebugType` "ForDuration" :`DrawTime` 0.1))
        (bind _asfire_old (cast `/Game/Blueprints/Scene/FireOld` (`.HitActor` (`GameplayStatics.BreakHitResult` _outhit))))
        (set `/Game/Blueprints/Scene/FireOld.Active` false _asfire_old)))))

(fn `UserConstructionScript`)